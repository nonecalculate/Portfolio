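; BP_GJNPC is an NPC that ragdolls, dissolves and is destroyed when its Health reaches zero.
; BeginPlay creates dynamic material instances on two mesh slots.
; Tick polls Health and, once, removes the right-fist collision box, enables mesh physics and disables capsule collision.
; A timeline then drives both materials' Dissolve parameter, with a five-second delay before destruction triggered from its update.
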(event EventBeginPlay
  (bind _mesh (Variables|Character|GetMesh))
  (bind _mesh_2 (Variables|Character|GetMesh))
  (bind _returnvalue (Rendering|Material|CreateDynamicMaterialInstance _mesh 0 "/Game/AI/Characters/Mannequins/Materials/Instances/Manny/MI_Manny_01.MI_Manny_01" "None" :!class /Script/Engine.PrimitiveComponent))
  (bind _output_get (Variables|Default|SetMaterial%20Instance _returnvalue))
  (bind _returnvalue_2 (Rendering|Material|CreateDynamicMaterialInstance _mesh 1 _output_get "None" :!class /Script/Engine.PrimitiveComponent))
  (Variables|Default|SetMaterial%20Instance1 _returnvalue_2)
  (Rendering|Material|SetMaterialbyName _mesh_2 "None" 0)
  (Rendering|Material|SetMaterialbyName _mesh_2 "None" 0))

(event EventTick
  (params (DeltaSeconds :type Float%20%28single-precision%29))
  (bind _mesh (Variables|Character|GetMesh))
  (if (<= (Variables|Default|GetHealth) 0.0)
    (Utilities|FlowControl|DoOnce false
      (:Completed
        (Components|DestroyComponent (Variables|Default|GetRightFistCollisionBox))
        (Physics|SetSimulatePhysics _mesh true)
        (Collision|SetCollisionProfileName _mesh "Ragdoll" true :!class /Script/Engine.PrimitiveComponent)
        (Collision|SetCollisionProfileName (Variables|Default|GetCapsuleComponent) "NoCollision" true :!class /Script/Engine.PrimitiveComponent)
        (bind _dissolve (Timeline|타임라인 Play)
          (:Update
            (Rendering|Material|SetScalarParameterValue (Variables|Default|GetMaterial%20Instance) "Dissolve" _dissolve :!class /Script/Engine.MaterialInstanceDynamic)
            (Utilities|FlowControl|Delay 5.0)
            (Actor|DestroyActor)))))))

(fn ConstructionScript)