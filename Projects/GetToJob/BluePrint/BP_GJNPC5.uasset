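; BP_GJNPC5 is an NPC Blueprint that handles its own death with a ragdoll and dissolve effect.
; BeginPlay creates a dynamic material instance on the mesh.
; Tick polls Health and, once it reaches zero, removes the right-fist collision box, switches the mesh to physics ragdoll and disables capsule collision.
; A timeline then drives the Dissolve parameter, with a delayed actor destroy chained from its update.
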(event EventBeginPlay
  (bind _returnvalue (Rendering|Material|CreateDynamicMaterialInstance (Variables|Character|GetMesh) 0 "/Game/AI/Scanned3DPeoplePack/RP_Character/rp_nathan_rigged_003_ue4/Materials/rp_nathan_rigged_003_mat.rp_nathan_rigged_003_mat" "None" :!class /Script/Engine.PrimitiveComponent))
  (Variables|Default|SetMaterial%20Instance _returnvalue)
  (Rendering|Material|SetMaterialbyName (Variables|Character|GetMesh) "None" 0))

(event EventTick
  (params (DeltaSeconds :type Float%20%28single-precision%29))
  (bind _mesh (Variables|Character|GetMesh))
  (if (<= (Variables|Default|GetHealth) 0.0)
    (Utilities|FlowControl|DoOnce false
      (:Completed
        (Components|DestroyComponent (Variables|Default|GetRightFistCollisionBox))
        (Physics|SetSimulatePhysics _mesh true)
        (Collision|SetCollisionProfileName _mesh "Ragdoll" true :!class /Script/Engine.PrimitiveComponent)
        (Collision|SetCollisionProfileName (Variables|Default|GetCapsuleComponent) "NoCollision" true :!class /Script/Engine.PrimitiveComponent)
        (bind _dissolve (Timeline|타임라인 Play)
          (:Update
            (Rendering|Material|SetScalarParameterValue (Variables|Default|GetMaterial%20Instance) "Dissolve" _dissolve :!class /Script/Engine.MaterialInstanceDynamic)
            (Utilities|FlowControl|Delay 5.0)
            (Actor|DestroyActor)))))))

(fn ConstructionScript)