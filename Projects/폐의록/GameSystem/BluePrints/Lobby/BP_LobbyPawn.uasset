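; BP_LobbyPawn is the lobby player pawn that hosts the inventory component for loading, saving, viewing and shop access.
; On BeginPlay, the local player polls until its unique net ID is valid, then uses it as the save-slot name.
; An existing BP_InventorySave is read client-side and sent to the server; otherwise the server is asked to save.
; Events toggle the inventory with cursor input, request saves and open named shops; consumed items are only logged.
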(event Custom|ToggleInTheShop)

(event Custom|Toggle%20In
  (bind _returnvalue (Game|GetPlayerController 0))
  (Default|ToggleInventory (Variables|Default|GetBP_InventoryComponent) 0 true)
  (Input|SetInputModeGameandUI _returnvalue 0 "DoNotLock" true false)
  (Variables|/Script/Engine.PlayerController|SetbShowMouseCursor _returnvalue true))

(event Custom|EnterTheShop
  (params (Shop%20Name :type Name))
  (Default|TryInteractionforShopper (Variables|Default|GetBP_InventoryComponent) Shop%20Name))

(event Custom|SaveDataInPawn
  (Default|SERVERRequestSaveData (Variables|Default|GetBP_InventoryComponent) (Utilities|String|Append (Class|AdvancedSessionsLibrary|UniqueNetIdtoString (Class|AdvancedSessionsLibrary|GetUniqueNetIDfromPlayerState (Variables|GetPlayerState))) "SaveData")))

(event Custom|DELG_OnItemConsumed_Event_0
  (params (Item :type S%20Rep%20Inv%20Info%20Structure))
  (Development|PrintString (Utilities|String|Append (Utilities|String|ToString(Name) (Utilities|Struct|BreakS_RepInvInfo Item)) " consumed!") false false))

(event EventBeginPlay
  (bind _playerstate (Variables|GetPlayerState))
  (bind _uniquenetid (Class|AdvancedSessionsLibrary|GetUniqueNetIDfromPlayerState _playerstate))
  (bind _string (Class|AdvancedSessionsLibrary|UniqueNetIdtoString _uniquenetid))
  (bind _returnvalue (Utilities|String|Append _string "SaveData"))
  (|CallParentFunction)
  (Utilities|FlowControl|Sequence
    (:then_0
      (EventDispatchers|AssignDELGonItemConsumed (Variables|Default|GetBP_InventoryComponent) (delegate Custom|DELG_OnItemConsumed_Event_0)))
    (:then_1
      (if (Pawn|IsLocallyControlled)
        (if (Class|AdvancedSessionsLibrary|IsValidUniqueNetID _uniquenetid) :!label _label
          (bind _returnvalue_2 (SaveGame|DoesSaveGameExist _returnvalue))
          (if _returnvalue_2
            (bind _returnvalue_3 (SaveGame|LoadGamefromSlot _returnvalue))
            (bind _asbp_inventory_save (Utilities|Casting|CastToBP_InventorySave _returnvalue_3))
            (Default|SERVERLoadClientSideData (Variables|Default|GetBP_InventoryComponent) _returnvalue (Variables|/Game/Assets/InventoryPickupSystem/System/SaveSystem/BP_InventorySave.BP_InventorySave_C|GetContainerUIDs _asbp_inventory_save) (Variables|/Game/Assets/InventoryPickupSystem/System/SaveSystem/BP_InventorySave.BP_InventorySave_C|GetItems _asbp_inventory_save))
            (else
              (Default|SERVERRequestSaveData (Variables|Default|GetBP_InventoryComponent) _returnvalue)))
          (else
            (Utilities|FlowControl|Delay 0.1)
            (goto _label)))))))

(fn ConstructionScript)