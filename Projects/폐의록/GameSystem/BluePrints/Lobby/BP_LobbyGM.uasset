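; Lobby game mode that seats connected players on lobby platforms and server-travels them to the main world map when the match starts.
; BeginPlay orders platforms by index tag; login and logout wait on that setup via a polling macro, then spawn or clear characters.
; Lobby info updates refresh the player's character, or ask the controller to retry, then flag on the first controller's UI whether all players are ready.
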(event EventBeginPlay
  (CallFunction|SetUpPlatforms))

(event EventPostLogin
  (params (NewPlayer :type Player%20Controller%20Object%20Reference))
  (Utilities|Array|Add (Variables|Default|GetPCs) NewPlayer)
  (Utilities|IfPlatformSetUpIsDone
    (:True
      (CallFunction|UpdatePlayeronPlatforms))))

(event EventOnLogout
  (params (ExitingController :type Controller%20Object%20Reference))
  (bind _asplayer_controller (Utilities|Casting|CastToPlayerController ExitingController))
  (Utilities|Array|RemoveItem (Variables|Default|GetPCs) _asplayer_controller)
  (Utilities|IfPlatformSetUpIsDone
    (:True
      (CallFunction|UpdatePlayeronPlatforms))))

(fn ConstructionScript)

(fn SetUpPlatforms
  (bind _outactors (Actor|GetAllActorsOfClass "/Game/GameSystem/BluePrints/Lobby/BP_LobbyPlatform.BP_LobbyPlatform_C"))
  (for _index (range 0 (Utilities|Array|LastIndex _outactors))
    (bind _outactors_2 (Actor|GetAllActorsOfClasswithTag "/Game/GameSystem/BluePrints/Lobby/BP_LobbyPlatform.BP_LobbyPlatform_C" (Utilities|String|StringToName (Utilities|String|ToString(Integer) _index))))
    (Utilities|Array|Add (Variables|Default|GetPlayerPlatforms) (Utilities|Array|Get(acopy) _outactors_2)))
  (Variables|Default|SetbPlatformsSetUpDone true))

(fn UpdatePlayeronPlatforms
  ;[0.15 0.15 0.15 0.5] Is PC Already Added In Platform
  (for _array_element (Variables|Default|GetPCs)
    (LocalVariables|SetLoop_PCAlreadyAdded false)
    (bind _array_element_2 (Utilities|Array|ForEachLoopwithBreak (Variables|Default|GetPlayerPlatforms) :!label _label)
      (:LoopBody
        (if (== (Variables|/Game/GameSystem/BluePrints/Lobby/BP_LobbyPlatform.BP_LobbyPlatform_C|GetPC _array_element_2) _array_element)
          (LocalVariables|SetLoop_PCAlreadyAdded true)
          (goto _label Break)))
      (:Completed
        ;[0.15 0.15 0.15 0.5] Add PC Platform
        (if (not (LocalVariables|GetLoop_PCAlreadyAdded))
          (bind _array_element_3 (Utilities|Array|ForEachLoopwithBreak (Variables|Default|GetPlayerPlatforms) :!label _label_2)
            (:LoopBody
              (Utilities|IsValid (Variables|/Game/GameSystem/BluePrints/Lobby/BP_LobbyPlatform.BP_LobbyPlatform_C|GetPC _array_element_3)
                (:Is%20Not%20Valid
                  (Default|SpawnCharacter _array_element_3 _array_element)
                  (goto _label_2 Break)))))))))
  ;[0.15 0.15 0.15 0.5] Remove disconnected Players from Platform
  (for _array_element_4 (Variables|Default|GetPlayerPlatforms)
    (if (not (Utilities|Array|ContainsItem (Variables|Default|GetPCs) (Variables|/Game/GameSystem/BluePrints/Lobby/BP_LobbyPlatform.BP_LobbyPlatform_C|GetPC _array_element_4)))
      (Default|Clear _array_element_4))))

(fn UpdatePlayerLobbInfo
  (params (RequestingPC :type Player%20Controller%20Object%20Reference))
  (for _array_element (Variables|Default|GetPlayerPlatforms)
    (if (== (Variables|/Game/GameSystem/BluePrints/Lobby/BP_LobbyPlatform.BP_LobbyPlatform_C|GetPC _array_element) RequestingPC)
      (bind _asbp_lobby_character (Utilities|Casting|CastToBP_LobbyCharacter (Variables|/Game/GameSystem/BluePrints/Lobby/BP_LobbyPlatform.BP_LobbyPlatform_C|GetCurrentCharacter _array_element)))
      (Default|UpdatePlayerLobbyInfo _asbp_lobby_character (Utilities|Struct|MakeS_PlayerLobbyInfo RequestingPC (Utilities|Text|ToText(String) (Class|AdvancedSessionsLibrary|GetPlayerName RequestingPC)) (.bReady (Utilities|Struct|BreakS_PlayerLobbyInfo (Variables|/Game/GameSystem/BluePrints/Lobby/BP_LobbyPC.BP_LobbyPC_C|GetPlayerLobbyInfoPC (.AsBP%20Lobby%20PC (Utilities|Casting|CastToBP_LobbyPC RequestingPC))))) (Variables|/Script/Engine.Controller|GetPlayerState RequestingPC)))
      (CallFunction|CheckifEnoughPlayersAreReady)
      (return)))
  (Default|TryAgainUpdatingLobbyInfo (.AsBP%20Lobby%20PC (Utilities|Casting|CastToBP_LobbyPC RequestingPC))))

(fn StartMatch
  (Class|AdvancedSessionsLibrary|ServerTravel "/Game/World/Maps/NewMainWoirld_WP" false false)
  (for _array_element (Variables|Default|GetPCs)
    (bind _asbp_lobby_pc (Utilities|Casting|CastToBP_LobbyPC _array_element))
    (Default|OnStartMatch _asbp_lobby_pc)))

(fn CheckifEnoughPlayersAreReady
  (LocalVariables|SetbAllPlayersReady true)
  (for _array_element (Variables|Default|GetPCs)
    (bind _asbp_lobby_pc (Utilities|Casting|CastToBP_LobbyPC _array_element))
    (if (not (.bReady (Utilities|Struct|BreakS_PlayerLobbyInfo (Variables|/Game/GameSystem/BluePrints/Lobby/BP_LobbyPC.BP_LobbyPC_C|GetPlayerLobbyInfoPC _asbp_lobby_pc))))
      (LocalVariables|SetbAllPlayersReady false)))
  (bind _asbp_lobby_pc_2 (Utilities|Casting|CastToBP_LobbyPC (Game|GetPlayerController 0)))
  (Variables|/Game/UI/Widget/Lobby/WBP_Lobby.WBP_Lobby_C|SetbEnoughPlayersReady (Variables|/Game/GameSystem/BluePrints/Lobby/BP_LobbyPC.BP_LobbyPC_C|GetLoobbie%20UI%20Ref _asbp_lobby_pc_2) (LocalVariables|GetbAllPlayersReady)))