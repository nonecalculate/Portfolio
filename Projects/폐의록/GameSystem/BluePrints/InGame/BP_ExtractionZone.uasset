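; Extraction zone actor that, once activated, lets an overlapping BP_PRCharacter_Girl extract and then destroys itself.
; Activation unhides the actor, enables overlap collision and attaches spark particles, with a multicast event mirroring this for clients.
; After a short delay, overlap polls until the player's unique net ID is valid.
; It then requests a server inventory save keyed by that ID, calls Extract on the PRPlayerState and destroys the zone.
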(event OnComponentBeginOverlap(Box)
  (params (OverlappedComponent :type Primitive%20Component%20Object%20Reference) (OtherActor :type Actor%20Object%20Reference) (OtherComp :type Primitive%20Component%20Object%20Reference) (OtherBodyIndex :type Integer) (bFromSweep :type Boolean) (SweepResult :type Hit%20Result%20Structure%20%28by%20ref%29))
  (bind _asbp_prcharacter_girl (Utilities|Casting|CastToBP_PRCharacter_Girl OtherActor))
  (Utilities|FlowControl|Delay 0.5)
  (Utilities|IsValid (.AsBP%20PRPlayer%20Controller (Utilities|Casting|CastToBP_PRPlayerController (Pawn|GetController _asbp_prcharacter_girl)))
    (:Is%20Valid
      (if (Class|AdvancedSessionsLibrary|IsValidUniqueNetID (Class|AdvancedSessionsLibrary|GetUniqueNetIDfromPlayerState (Variables|/Script/Engine.Controller|GetPlayerState (.AsBP%20PRPlayer%20Controller (Utilities|Casting|CastToBP_PRPlayerController (Pawn|GetController _asbp_prcharacter_girl)))))) :!label _label
        (Default|SERVERRequestSaveData (Variables|/Game/Character/BP_BasePRCharacter.BP_BasePRCharacter_C|GetBP_InventoryComponent _asbp_prcharacter_girl) (Utilities|String|Append (Class|AdvancedSessionsLibrary|UniqueNetIdtoString (Class|AdvancedSessionsLibrary|GetUniqueNetIDfromPlayerState (Variables|/Script/Engine.Controller|GetPlayerState (.AsBP%20PRPlayer%20Controller (Utilities|Casting|CastToBP_PRPlayerController (Pawn|GetController _asbp_prcharacter_girl)))))) "SaveData"))
        (Development|PrintString "Overlapped" false)
        (bind _asprplayer_state (Utilities|Casting|CastToPRPlayerState (Variables|/Script/Engine.Pawn|GetPlayerState _asbp_prcharacter_girl)))
        (Class|PRPlayerState|Extract _asprplayer_state)
        (Actor|DestroyActor)
        (else
          (Utilities|FlowControl|Delay 0.1)
          (goto _label))))))

(event Custom|ActivateZone
  (Development|PrintString "Activated!" false)
  (Rendering|SetActorHiddenInGame false)
  (Collision|SetCollisionProfileName (Variables|Default|GetBox) "OverlapAll" true :!class /Script/Engine.PrimitiveComponent)
  (Effects|SpawnEmitterAttached "/Game/StarterContent/Particles/P_Sparks.P_Sparks" (Variables|Default|GetStaticMesh) "None")
  (CallFunction|MulticastActivateZone))

(event Custom|Multicast_ActivateZone
  (Rendering|SetActorHiddenInGame false)
  (Collision|SetCollisionProfileName (Variables|Default|GetBox) "OverlapAll" true :!class /Script/Engine.PrimitiveComponent)
  (Effects|SpawnEmitterAttached "/Game/StarterContent/Particles/P_Sparks.P_Sparks" (Variables|Default|GetStaticMesh) "None"))

(fn ConstructionScript)