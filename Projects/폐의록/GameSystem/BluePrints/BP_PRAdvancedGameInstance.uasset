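; Advanced game instance that manages multiplayer session creation, update and teardown, with Steam named in the failure warning.
; CreateSession opens an eight-slot session and travels to Lobby as a listen server, or shows a warning popup on failure.
; UpdateSession closes public slots and stops advertising, while DestroySession returns to TempMainMenu on success.
; Shutdown is empty, and an unconnected inventory save-loading fragment never runs.
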(event Custom|CreateSession
  (|AdvancedSession 0 (Game|GetPlayerController 0) 8 0 false true false true true false false false true false true
    (:OnSuccess
      (Game|OpenLevel(byObjectReference) "/Game/World/Maps/Lobby.Lobby" true "listen"))
    (:OnFailure
      (bind _returnvalue (UserInterface|CreateWidget "/Game/Item/Shop/WBP_Popup.WBP_Popup_C" (Game|GetPlayerController 0)))
      (Rendering|Components|TextRender|SetText (Variables|/Game/Item/Shop/WBP_Popup.WBP_Popup_C|GetWarning _returnvalue) "용병단 창설에 실패했습니다. 
스팀이 꺼져 있는 경우 게임을 종료한 뒤 
스팀을 실행하고 다시 시작해주세요.")
      (UserInterface|Viewport|AddtoViewport _returnvalue 0))))

(event Custom|Destroy%20Session
  (|DestroySession (Game|GetPlayerController 0)
    (:OnSuccess
      (Development|PrintString "SessionDestroyed")
      (Game|OpenLevel(byObjectReference) "/Game/GameSystem/Levels/TempMainMenu.TempMainMenu"))
    (:OnFailure
      (Development|PrintString "Cannot Destroy Session"))))

(event Custom|UpdateSession
  (|UpdateSession 0 0 0 false false false true false false))

(event EventShutdown)