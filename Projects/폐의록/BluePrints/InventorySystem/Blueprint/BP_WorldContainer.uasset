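; World container actor that holds items in an inventory component and exposes the GUID of its widget's first container.
; Outside dedicated servers, BeginPlay binds the interact delegate, plays the chest spawn sound and snaps the actor to the surface found by a downward trace.
; The interact delegate shows or clears a name widget.
; Item add and remove events call multicasts that keep the Niagara effect active only while the inventory has items.
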(event DELGonItemAdded(BP_InventoryComponent)
  (params (ContainerName :type Name :default "None") (Item :type S%20Rep%20Inv%20Info%20Structure) (Actor :type Actor%20Object%20Reference))
  ;[0.15 0.15 0.15 0.5] 나이아가라 ON/OFF
  (bind _invitems (Default|GetInvItems (Variables|Default|GetBP_InventoryComponent)))
  (if (Utilities|Array|IsEmpty _invitems)
    (CallFunction|MulticastSetNiagaraDeactivate)
    (else
      (CallFunction|MulticastSetNiagaraActivate))))

(event DELGonItemRemoved(BP_InventoryComponent)
  (params (ContainerName :type Name :default "None") (Info :type S%20Rep%20Inv%20Info%20Structure))
  ;[0.15 0.15 0.15 0.5] 나이아가라 ON/OFF
  (bind _invitems (Default|GetInvItems (Variables|Default|GetBP_InventoryComponent)))
  (if (Utilities|Array|IsEmpty _invitems)
    (CallFunction|MulticastSetNiagaraDeactivate)
    (else
      (CallFunction|MulticastSetNiagaraActivate))))

(event Custom|DELG_ContainerInteraction_Event_0
  (params (Value :type Boolean))
  (bind _widget (Variables|Default|GetWidget))
  (if Value
    (bind _returnvalue (UserInterface|CreateWidget "/Game/Assets/InventoryPickupSystem/System/PickupSystem/UI_PickupItemName.UI_PickupItemName_C"))
    (UserInterface|SetWidget _widget _returnvalue)
    (Default|UpdateName _returnvalue (Variables|Settings|GetContainerName) "(TagName=\"Inv.Rarity.Common\")")
    (else
      (UserInterface|SetWidget _widget 0))))

(event Custom|Multicast_PlayChestSound
  ;[0.15 0.15 0.15 0.5] 상자생성사운드
  (Audio|PlaySoundatLocation (Variables|Default|GetSound) (Transformation|GetActorLocation) "0, 0, 0" 1.0 1.0 0.0 "/Game/Character/Sound/HitSoundAttenuation.HitSoundAttenuation" 0 0 0))

(event Custom|Multicast_SetNiagaraActivate
  ;[0.15 0.15 0.15 0.5] 나이아가라 ON/OFF
  (Components|Activation|Activate (Variables|Default|GetNiagara) true))

(event Custom|Multicast_SetNiagaraDeactivate
  ;[0.15 0.15 0.15 0.5] 나이아가라 ON/OFF
  (Components|Activation|Deactivate (Variables|Default|GetNiagara)))

(event EventBeginPlay
  (bind _returnvalue (Transformation|GetActorLocation))
  (if (not (Networking|IsDedicatedServer))
    (EventDispatchers|BindEventtoDELGContainerInteract (Variables|Default|GetBP_InventoryComponent) (delegate Custom|DELG_ContainerInteraction_Event_0))
    (CallFunction|MulticastPlayChestSound)
    (bind _outhit (Collision|LineTraceByChannel (+ _returnvalue "0.000000,0.000000,100.000000") (- _returnvalue "0.000000,0.000000,300.000000") "TraceTypeQuery1" false 0 "None"))
    (Transformation|SetActorLocation (.Location (Collision|BreakHitResult _outhit)) false false)))

(fn ConstructionScript)

(fn GetContainerUID
  (bind _containers (Default|GetListOfContainers (Default|GetInventoryWidget (Variables|Default|GetBP_InventoryComponent))))
  (return (Default|GetGUID (Utilities|Array|Get(acopy) _containers))))