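; BP_InvLib is a helper library for the inventory system, covering item data lookup, rarity colors and random stat rolls.
; GetInventoryData finds an item by ID in a data asset, and GetColorFromRarity maps rarity gameplay tags to colors, defaulting to white.
; GetRandStats walks the item's RollStats in order, adding each that passes its percent chance with random in-range values, optionally truncated to integers, until MaxStats is reached.
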(fn GetInventoryData
  (params (ID :type Name))
  (bind (_value _found_) (Default|FindItem (LocalVariables|GetDA) ID))
  (return _value _found_))

(fn GetColorfromRarity
  (params (Tag :type Gameplay%20Tag%20Structure))
  (|SwitchGameplayTag Tag
    (:Default
      (return "(R=1.000000,G=1.000000,B=1.000000,A=1.000000)"))
    (:Inv.Rarity.Common
      (return "(R=0.200000,G=0.200000,B=0.200000,A=1.000000)"))
    (:Inv.Rarity.Rare
      (return "(R=0.184896,G=0.186946,B=0.739583,A=1.000000)"))
    (:Inv.Rarity.Epic
      (return "(R=0.791667,G=0.174719,B=0.261657,A=1.000000)"))
    (:Inv.Rarity.Legendary
      (return "(R=0.843750,G=0.463509,B=0.140625,A=1.000000)"))))

(fn GetRandStats
  (params (ID :type Name))
  (bind _result (LocalVariables|GetResult))
  (bind _value (CallFunction|GetInventoryData ID))
  (Utilities|FlowControl|Sequence
    (:then_0
      (for _index (range 0 (Utilities|Array|LastIndex (.RollStats (Utilities|Struct|BreakS_InvItemInfo _value))))
        (if (<= (Math|Random|RandomFloatinRange 0.0 1e+02) (.Chance (Utilities|Struct|BreakS_InvStat (Utilities|Array|Get(acopy) (.RollStats (Utilities|Struct|BreakS_InvItemInfo _value)) _index))))
          (Utilities|Array|Add _result (Utilities|Struct|MakeS_RepStat (.Tag (Utilities|Struct|BreakS_InvStat (Utilities|Array|Get(acopy) (.RollStats (Utilities|Struct|BreakS_InvItemInfo _value)) _index))) (Math|Float|SelectFloat (Math|Conversions|ToFloat(Integer) (Math|Float|Truncate (Math|Random|RandomFloatinRange (.Min (Utilities|Struct|BreakS_InvStat (Utilities|Array|Get(acopy) (.RollStats (Utilities|Struct|BreakS_InvItemInfo _value)) _index))) (.Max (Utilities|Struct|BreakS_InvStat (Utilities|Array|Get(acopy) (.RollStats (Utilities|Struct|BreakS_InvItemInfo _value)) _index)))))) (Math|Random|RandomFloatinRange (.Min (Utilities|Struct|BreakS_InvStat (Utilities|Array|Get(acopy) (.RollStats (Utilities|Struct|BreakS_InvItemInfo _value)) _index))) (.Max (Utilities|Struct|BreakS_InvStat (Utilities|Array|Get(acopy) (.RollStats (Utilities|Struct|BreakS_InvItemInfo _value)) _index)))) (.ConvertToInt? (Utilities|Struct|BreakS_InvStat (Utilities|Array|Get(acopy) (.RollStats (Utilities|Struct|BreakS_InvItemInfo _value)) _index)))) (Math|Float|SelectFloat (Math|Conversions|ToFloat(Integer) (Math|Float|Truncate (Math|Random|RandomFloatinRange (.Min (Utilities|Struct|BreakS_InvStat (Utilities|Array|Get(acopy) (.RollStats (Utilities|Struct|BreakS_InvItemInfo _value)) _index))) (.Max (Utilities|Struct|BreakS_InvStat (Utilities|Array|Get(acopy) (.RollStats (Utilities|Struct|BreakS_InvItemInfo _value)) _index)))))) (Math|Random|RandomFloatinRange (.Min (Utilities|Struct|BreakS_InvStat (Utilities|Array|Get(acopy) (.RollStats (Utilities|Struct|BreakS_InvItemInfo _value)) _index))) (.Max (Utilities|Struct|BreakS_InvStat (Utilities|Array|Get(acopy) (.RollStats (Utilities|Struct|BreakS_InvItemInfo _value)) _index)))) (.ConvertToInt? (Utilities|Struct|BreakS_InvStat (Utilities|Array|Get(acopy) (.RollStats (Utilities|Struct|BreakS_InvItemInfo _value)) _index))))))
          (if (>= (Utilities|Array|Length _result) (.MaxStats (Utilities|Struct|BreakS_InvItemInfo _value)))
            (return (LocalVariables|GetResult))))))
    (:then_1
      (return (LocalVariables|GetResult)))))