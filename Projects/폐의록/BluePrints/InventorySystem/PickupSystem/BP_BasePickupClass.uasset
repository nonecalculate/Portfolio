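; BP_BasePickupClass is the base Blueprint for pickups, showing an item name label in response to pickup interaction.
; On BeginPlay, outside dedicated servers, it binds to the interaction delegate of its BPPickupComponent.
; A true value creates a UI_PickupItemName widget in the Widget component and fills it with the component's item name and rarity.
; A false value clears the widget.
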(event Custom|DELG_PickupInteraction_Event_0
  (params (Value :type Boolean))
  (bind _widget (Variables|Default|GetWidget))
  (bind _bp_pickupcomponent (Variables|Default|GetBP_PickupComponent))
  (if Value
    (bind _returnvalue (UserInterface|CreateWidget "/Game/Assets/InventoryPickupSystem/System/PickupSystem/UI_PickupItemName.UI_PickupItemName_C"))
    (UserInterface|SetWidget _widget _returnvalue)
    (Default|UpdateName _returnvalue (Default|GetItemName _bp_pickupcomponent) (Default|GetRarity _bp_pickupcomponent))
    (else
      (UserInterface|SetWidget _widget 0))))

(event EventBeginPlay
  (if (not (Networking|IsDedicatedServer))
    (EventDispatchers|AssignDELGPickupInteraction (Variables|Default|GetBP_PickupComponent) (delegate Custom|DELG_PickupInteraction_Event_0))))

(fn ConstructionScript)