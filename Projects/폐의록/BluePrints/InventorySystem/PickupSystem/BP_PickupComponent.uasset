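; Pickup component that makes its owning actor an inventory item, serving item data, count, rarity, stats and container persistence data.
; On BeginPlay it caches data by ItemID; the authority rolls rarity, stats and count, adding more non-duplicate random stats at higher rarities when base stats exist.
; OnRep handlers broadcast count, rarity and interactability changes through delegates.
; Pickup destroys the actor, or disables interaction for equipped items not flagged DestroyWhenEquipped.
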(event EventBeginPlay
  (bind _cachedinfo (Variables|Default|GetCachedInfo))
  (bind _statsstring (Variables|Default|GetStatsString))
  (bind (_possiblerarities _defaultcount) (Utilities|Struct|BreakS_InvItemInfo _cachedinfo))
  (CallFunction|CachInfo)
  (if (Ability|HasAuthority (Components|GetOwner))
    (bind _output_get (Variables|Default|SetRepRarity (.OutItem (Utilities|Array|Random (GameplayTags|BreakGameplayTagContainer _possiblerarities)))))
    (bind _output_get_2 (Variables|Default|SetStats (CallFunction|GetRandStats (Variables|Settings|GetItemID))))
    (for _array_element _output_get_2
      (Utilities|Array|Add _statsstring (GameplayTags|GetDebugStringfromGameplayTag (.Tag (Utilities|Struct|BreakS_RepStat _array_element)))))
    (if (Utilities|Array|IsEmpty _statsstring)
      _
      (else
        (switch string (GameplayTags|GetDebugStringfromGameplayTag _output_get)
          (:Default
            _)
          (:Inv.Rarity.Common
            _)
          (:Inv.Rarity.Rare
            (CallFunction|MakeRandomStats (Variables|Default|GetStats) (Variables|Default|GetStatsString)))
          (:Inv.Rarity.Epic
            (CallFunction|MakeRandomStats (Variables|Default|GetStats) (Variables|Default|GetStatsString) 1))
          (:Inv.Rarity.Legendary
            (CallFunction|MakeRandomStats (Variables|Default|GetStats) (Variables|Default|GetStatsString) 2)))))
    (if (> (Variables|Settings|GetOverrideCount) 0)
      (Variables|Default|SetRepCount (Variables|Settings|GetOverrideCount))
      (else
        (Variables|Default|SetRepCount _defaultcount)))))

(fn GetInfo
  (CallFunction|CachInfo)
  (return (Variables|Default|GetCachedInfo) true))

(fn SetPickupInteractionEnabled
  (params (Value :type Boolean))
  (bind _as프리미티브_컴포넌트 (Utilities|Casting|CastToPrimitiveComponent (Variables|/Script/Engine.Actor|GetRootComponent (Components|GetOwner))))
  (Collision|SetCollisionEnabled _as프리미티브_컴포넌트 (select Value "QueryAndPhysics" "NoCollision"))
  (Physics|SetSimulatePhysics _as프리미티브_컴포넌트 Value))

(fn OnPickupInteraction
  (params (Value :type Boolean))
  (Default|CallDELGPickupInteraction Value))

(fn OnRepCanInteract?
  (CallFunction|OnPickupInteraction (Variables|Default|GetCanInteract?))
  (Default|CallDELGRepInfoUpdated))

(fn SetCanInteract
  (params (CanInteract? :type Boolean))
  (Variables|Default|SetCanInteract? CanInteract?))

(fn GetCanInteract
  (return (Variables|Default|GetCanInteract?)))

(fn GetItemName
  (bind _repcount (Variables|Default|GetRepCount))
  (return (Utilities|Text|FormatText "{name}{count}" (.Name (Utilities|Struct|BreakS_InvItemInfo (Variables|Default|GetCachedInfo))) (select (> _repcount 1) (Utilities|Text|FormatText " x{count}" _repcount) ""))))

(fn OnRepRepCount
  (Default|CallDELGRepInfoUpdated))

(fn GetCount
  (return (Variables|Default|GetRepCount)))

(fn GetRarity
  (return (Variables|Default|GetRepRarity)))

(fn OnRepRepRarity
  (Default|CallDELGRepInfoUpdated))

(fn GetDurability
  (bind _value (CallFunction|GetInfo))
  (return (Math|Random|RandomFloatinRange (.X (Math|Vector2D|BreakVector2D (.RandomDurability (Utilities|Struct|BreakS_InvItemInfo _value)))) (.Y (Math|Vector2D|BreakVector2D (.RandomDurability (Utilities|Struct|BreakS_InvItemInfo _value)))))))

(fn GetCapacity
  (bind _value (CallFunction|GetInfo))
  (return (.MaxCapacity (Utilities|Struct|BreakS_InvItemInfo _value))))

(fn GetStats
  (return (Variables|Default|GetStats)))

(fn GetDimension
  (bind _value (CallFunction|GetInfo))
  (return (.Dimention (Utilities|Struct|BreakS_InvItemInfo _value))))

(fn OnPickedUp
  (params (Owner :type Actor%20Object%20Reference) (Equipped? :type Boolean))
  (if Equipped?
    (bind _value (CallFunction|GetInfo))
    (if (.DestroyWhenEquipped? (Utilities|Struct|BreakS_InvItemInfo _value))
      (Actor|DestroyActor (Components|GetOwner))
      (else
        (CallFunction|SetCanInteract false)))
    (else
      (Actor|DestroyActor (Components|GetOwner)))))

(fn CachInfo
  (if (== (.ID (Utilities|Struct|BreakS_InvItemInfo (Variables|Default|GetCachedInfo))) "")
    (bind _value (CallFunction|GetInventoryData (Variables|Settings|GetItemID)))
    (Variables|Default|SetCachedInfo _value)))

(fn GetMaxStack
  (bind _cachedinfo (Variables|Default|GetCachedInfo))
  (bind (_canstack_ _maxstack) (Utilities|Struct|BreakS_InvItemInfo _cachedinfo))
  (return _canstack_ _maxstack))

(fn SetCount
  (params (NewCount :type Integer))
  (Variables|Default|SetRepCount NewCount))

(fn SetPickupPersistentData
  (params (GUID :type Guid%20Structure) (Content :type Array%20of%20S%20Rep%20Inv%20Info%20Structures))
  (Variables|Default|SetGUID GUID)
  (Variables|Default|SetContent Content))

(fn GetPersistentData
  (return (Variables|Default|GetGUID) (Variables|Default|GetContentGUID) (Variables|Default|GetContent)))

(fn IsContainer?
  (bind _cachedinfo (Variables|Default|GetCachedInfo))
  (bind _containerslots (Utilities|Struct|BreakS_InvItemInfo _cachedinfo))
  (bind (_x _y) (Utilities|Struct|BreakIntPoint _containerslots))
  (return (> (+ _x _y) 1) _containerslots))

(fn SetRarity
  (params (RepRarity :type Gameplay%20Tag%20Structure))
  (Variables|Default|SetRepRarity RepRarity))

(fn SetStats
  (params (Stats :type Array%20of%20S%20Rep%20Stat%20Structures))
  (Variables|Default|SetStats Stats))

(fn MakeRandomStats
  (params (Stats :type Array%20of%20S%20Rep%20Stat%20Structures) (ExistStats :type Array%20of%20Strings) (Rairity :type Integer))
  (for _index (range 0 Rairity)
    (LocalVariables|SetIsStatExisted? false)
    (bind (_randomstat _statstring _returnvalue) (CallFunction|RandomStat))
    (bind _array_element (Utilities|Array|ForEachLoopwithBreak ExistStats :!label _label)
      (:LoopBody
        (bind _output_get (LocalVariables|SetIsStatExisted? (Utilities|Enum|Equal(Enum) _statstring _array_element)))
        (if _output_get
          (goto _label Break)))
      (:Completed
        (if (LocalVariables|GetIsStatExisted?)
          (Math|Integer|DecrementInt _index)
          (else
            (Utilities|Array|Add (Variables|Default|GetStats) (Utilities|Struct|MakeS_RepStat _randomstat (Math|Conversions|ToFloat(Integer) _returnvalue) (Math|Conversions|ToFloat(Integer) _returnvalue)))
            (Utilities|Array|Add ExistStats (GameplayTags|GetDebugStringfromGameplayTag _randomstat)))))))
  (return))

(fn RandomStat
  (bind _statuscontainer (Variables|Default|GetStatusContainer))
  (bind _stats (Utilities|Struct|BreakS_Stats _statuscontainer))
  (bind _gameplaytags (GameplayTags|BreakGameplayTagContainer _stats))
  (bind _outitem (Utilities|Array|Random _gameplaytags))
  (return _outitem (GameplayTags|GetDebugStringfromGameplayTag _outitem) (Math|Random|RandomIntegerinRange 1 4)))

(fn SetValue
  (params (Value :type Name))
  (Variables|Default|SetValue (Math|Conversions|ToInteger(Byte) (Class|KismetMathLibrary|ToInt64(Float) (.SellValue (Utilities|Struct|BreakS_InvItemInfo (Variables|Default|GetCachedInfo)))))))

(fn GetValue
  (return (Variables|Default|GetValue)))

(fn OnRepValue)