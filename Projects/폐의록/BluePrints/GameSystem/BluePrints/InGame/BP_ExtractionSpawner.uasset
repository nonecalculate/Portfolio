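; BP_ExtractionSpawner is a placed spawner actor that spawns an instance of its WantToSpawn class when play begins, apparently an extraction crate.
; BeginPlay calls the server-named spawn event, which uses the Arrow component's world location and scale but not its rotation.
; Spawning adjusts for collisions but always succeeds.
; A client-named event duplicates the same spawn logic and is not called within this Blueprint.
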(event Custom|Serve_Spawn%20Crate
  (bind _arrow (Variables|Default|GetArrow))
  (bind _returnvalue (Transformation|GetWorldTransform _arrow))
  (bind (_location _rotation _scale) (Math|Transform|BreakTransform _returnvalue))
  (Game|SpawnActorfromClass (Variables|Default|GetWantToSpawn) (Math|Transform|MakeTransform _location "0, 0, 0" _scale) "AdjustIfPossibleButAlwaysSpawn" "MultiplyWithRoot" 0 0))

(event Custom|Client_Spawn%20Crate
  (bind _arrow (Variables|Default|GetArrow))
  (bind _returnvalue (Transformation|GetWorldTransform _arrow))
  (bind (_location _rotation _scale) (Math|Transform|BreakTransform _returnvalue))
  (Game|SpawnActorfromClass (Variables|Default|GetWantToSpawn) (Math|Transform|MakeTransform _location "0, 0, 0" _scale) "AdjustIfPossibleButAlwaysSpawn" "MultiplyWithRoot" 0 0))

(event EventBeginPlay
  (CallFunction|ServeSpawnCrate))

(fn ConstructionScript)