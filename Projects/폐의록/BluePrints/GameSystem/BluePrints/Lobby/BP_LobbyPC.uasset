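; Player controller for the multiplayer lobby, handling lobby UI, player name and ready status.
; On the local client, setup shows the Lobby widget and sends the GameInstance's player name to the server, while BeginPlay plays ambient insect sound.
; Name and ready changes update the player's lobby struct and push it to BP_LobbyGM, with a delayed retry event.
; Client events show loading at match start and save clothes color.
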(event Custom|TryAgainUpdatingLobbyInfo
  (Utilities|FlowControl|Delay 0.1)
  (bind _asbp_lobby_gm (Utilities|Casting|CastToBP_LobbyGM (Game|GetGameMode)))
  (Default|UpdatePlayerLobbInfo _asbp_lobby_gm self))

(event Custom|SetPlayerNameOnServer
  (params (PlayerName :type Text))
  (Utilities|Struct|SetmembersinS_PlayerLobbyInfo (Variables|Default|GetPlayerLobbyInfoPC) PlayerName)
  (bind _asbp_lobby_gm (Utilities|Casting|CastToBP_LobbyGM (Game|GetGameMode)))
  (Default|UpdatePlayerLobbInfo _asbp_lobby_gm self))

(event Custom|OnStartMatch
  (Class|UIManager|ShowWidget (Subsystems|GetUIManager) "Loading")
  (Input|DisableInput self))

(event Custom|ToggleReadyStatusOnServer
  (bind _playerlobbyinfopc (Variables|Default|GetPlayerLobbyInfoPC))
  (Utilities|Struct|SetmembersinS_PlayerLobbyInfo _playerlobbyinfopc (not (.bReady (Utilities|Struct|BreakS_PlayerLobbyInfo _playerlobbyinfopc))))
  (bind _asbp_lobby_gm (Utilities|Casting|CastToBP_LobbyGM (Game|GetGameMode)))
  (Default|UpdatePlayerLobbInfo _asbp_lobby_gm self))

(event Custom|Client_SaveColor
  (params (Color :type Linear%20Color%20Structure))
  (Class|SaveDataSubsystem|SetClothesColor (Subsystems|GetSaveDataSubsystem) Color))

(event EventBeginPlay
  (CallFunction|SetUp)
  (if (Pawn|IsLocalController)
    (Audio|PlaySound2D "/Game/Assets/Sounds/Atmosphere/Sound_Background_SummerInsects.Sound_Background_SummerInsects" 1.0 1.0 0.0 0 0)))

(event Input|ActionEvents|InputActionUI_Escape
  (params (Key :type Key%20Structure :default "None"))
  ;[0.15 0.15 0.15 0.5] 버튼이 안사라지고, Stash 는 안먹힘 가호는 먹히는데
)

(fn ConstructionScript)

(fn SetUp
  (bind _returnvalue (Subsystems|GetUIManager))
  (if (Pawn|IsLocalPlayerController)
    (Variables|Default|SetbShowMouseCursor true)
    (Input|SetInputModeGameandUI self 0 "DoNotLock" false false)
    (Class|UIManager|RemoveAllWidgets _returnvalue)
    (bind _returnvalue_2 (Class|UIManager|ShowWidget _returnvalue "Lobby"))
    (bind _aswbp_lobby (Utilities|Casting|CastToWBP_Lobby _returnvalue_2))
    (Variables|Default|SetLoobbie%20UI%20Ref _aswbp_lobby)
    (CallFunction|SetPlayerNameonServer (Utilities|Text|ToText(Name) (Utilities|String|StringToName (Variables|/Game/GameSystem/BluePrints/BP_PRAdvancedGameInstance.BP_PRAdvancedGameInstance_C|GetPlayerName (.AsBP%20PRAdvanced%20Game%20Instance (Utilities|Casting|CastToBP_PRAdvancedGameInstance (Game|GetGameInstance)))))))))