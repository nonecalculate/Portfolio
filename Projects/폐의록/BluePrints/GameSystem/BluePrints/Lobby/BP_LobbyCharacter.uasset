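; BP_LobbyCharacter is the character displayed in the lobby, showing a player's info widget, clothes color and animation.
; Each is driven by a RepNotify variable, with UpdatePlayerLobbyInfo setting the player info.
; The info notify updates and reveals the WB_PlayerLobbyInfo widget, retrying on a short timer until that widget is valid.
; The other notifies tint a dynamic material instance on the mesh and play the assigned looping animation.
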(fn ConstructionScript)

(fn UpdatePlayerLobbyInfo
  (params (PlayerLobbyInfo :type S%20Player%20Lobby%20Info%20Structure))
  (Variables|Default|SetPlayerLobbyInfo PlayerLobbyInfo))

(fn OnRepPlayerLobbyInfo
  (bind _lobbyinfo (Variables|Default|GetLobbyInfo))
  (bind _returnvalue (UserInterface|GetWidget _lobbyinfo))
  (Utilities|IsValid _returnvalue
    (:Is%20Valid
      (bind _aswb_player_lobby_info (Utilities|Casting|CastToWB_PlayerLobbyInfo _returnvalue))
      (Default|Update _aswb_player_lobby_info (Variables|Default|GetPlayerLobbyInfo))
      (Rendering|SetVisibility (Variables|Default|GetLobbyInfo) true false))
    (:Is%20Not%20Valid
      (Utilities|Time|SetTimerbyFunctionName 0 "OnRep_PlayerLobbyInfo" 0.1))))

(fn OnRepClothesColor
  (bind _returnvalue (Rendering|Material|CreateDynamicMaterialInstance (Variables|Character|GetMesh) 6 0 "None" :!class /Script/Engine.PrimitiveComponent))
  (Rendering|Material|SetVectorParameterValue _returnvalue "[4] To Texture Color" (Variables|Default|GetClothesColor) :!class /Script/Engine.MaterialInstanceDynamic))

(fn OnRepAnimtoPlay
  (bind _mesh (Variables|Character|GetMesh))
  (Components|Animation|SetAnimation _mesh (Variables|Default|GetAnimToPlay))
  (Audio|Components|Audio|Play _mesh true))