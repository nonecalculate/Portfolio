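; BP_LobbyPC is the lobby player controller that connects the game mode to each player's lobby UI and chat.
; It creates the lobby widget with server details, forwards player list and count updates to it, and swaps it for a loading screen.
; Chat messages are tagged with the player's name, sent through every controller in BP_LobbyGM's list and saved to its history.
; Kicking opens the Menu level and destroys the session.
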(event Custom|AddLobbyWB
  (params (ServerName :type String) (ServerMap :type String) (ServerMode :type String) (ServerSlots :type Integer))
  (Variables|Default|SetbShowMouseCursor true)
  (bind _returnvalue (UserInterface|CreateWidget "/Game/GameMode/UMG/UMG_Lobby.UMG_Lobby_C" 0 (Utilities|Text|ToText(String) ServerName) (Utilities|Text|ToText(String) ServerMap) (Utilities|Text|ToText(String) ServerMode) ServerSlots))
  (bind _output_get (Variables|Default|SetLobbyWB _returnvalue))
  (UserInterface|Viewport|AddtoViewport _output_get 1))

(event Custom|LoadingScreen
  (Widget|RemovefromParent (Variables|Default|GetLobbyWB))
  (bind _returnvalue (UserInterface|CreateWidget "/Game/GameMode/UMG/UMG_LoadingScreen.UMG_LoadingScreen_C" self))
  (UserInterface|Viewport|AddtoViewport _returnvalue 0))

(event Custom|AddPlayer
  (params (Player :type Text) (PlayerIndex :type Integer))
  (Default|AddPlayertoList (Variables|Default|GetLobbyWB) Player PlayerIndex))

(event Custom|ClearPlayerList
  (Default|ClearPlayerList (Variables|Default|GetLobbyWB)))

(event Custom|KickPlayer
  (Game|OpenLevel(byName) "Menu")
  (|DestroySession self))

(event Custom|UpdateNumberOfPlayers
  (params (CurrentPlayers :type Integer))
  (Variables|/Game/GameMode/UMG/UMG_Lobby.UMG_Lobby_C|SetCurrentPlayers (Variables|Default|GetLobbyWB) CurrentPlayers))

(event Custom|AddMessageFromServerToEachPlayer
  (params (Message :type String) (Color :type Slate%20Color%20Structure) (isServerMessage? :type Boolean))
  (bind _self self)
  (bind _playername (Class|AdvancedSessionsLibrary|GetPlayerName _self))
  (bind _chatmessagestructure (Utilities|Struct|MakeChatMessageStructure _playername Message Color isServerMessage?))
  (bind _asbp_lobby_gm (Utilities|Casting|CastToBP_LobbyGM (Game|GetGameMode)))
  (for _array_element (Variables|/Game/GameMode/Blueprints/BP_LobbyGM.BP_LobbyGM_C|GetAllPCs _asbp_lobby_gm)
    (bind _asbp_lobby_pc (Utilities|Casting|CastToBP_LobbyPC _array_element))
    (CallFunction|AddMessagetoChat _asbp_lobby_pc _chatmessagestructure))
  (bind _asbp_lobby_gm_2 (Utilities|Casting|CastToBP_LobbyGM (Game|GetGameMode)))
  (Default|AddMessagetoChatHistory _asbp_lobby_gm_2 _chatmessagestructure))

(event Custom|AddMessageToChat
  (params (ChatMessageStructure :type Chat%20Message%20Structure%20Structure))
  (Default|AddChildtoChat (Variables|/Game/GameMode/UMG/UMG_Lobby.UMG_Lobby_C|GetUMG_ChatWindow (Variables|Default|GetLobbyWB)) ChatMessageStructure))

(fn ConstructionScript)