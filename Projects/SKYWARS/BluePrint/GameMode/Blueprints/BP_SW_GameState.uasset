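; BP_SW_GameState is the game state Blueprint for the SKYWARS mode, recording the order in which players die.
; Its AddRanking event maps the dead player's name to the current Players counter in PlayerRankingList, then increments the counter.
; It then prints every name with its key-array index and a "Grades" label as on-screen debug output, rather than printing the stored rank.
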(event EventAddRanking
  (params (DeadUserPC :type Player%20Controller%20Object%20Reference))
  (bind _players (Variables|Default|GetPlayers))
  (Utilities|Map|Add (Variables|Default|GetPlayerRankingList) (Class|AdvancedSessionsLibrary|GetPlayerName DeadUserPC) _players)
  (Math|Integer|IncrementInt _players
    (:%20%20
      (bind _keys (Utilities|Map|Keys (Variables|Default|GetPlayerRankingList)))
      (for (_array_element _array_index) _keys
        (Development|PrintString (Utilities|String|Append _array_element ": " (Utilities|String|ToString(Integer) _array_index) " Grades"))))))

(fn ConstructionScript)