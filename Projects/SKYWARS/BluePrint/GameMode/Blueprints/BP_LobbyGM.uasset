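; Lobby game mode for SKYWARS that tracks player controllers, relays chat and kicks players.
; PostLogin announces joins, builds each lobby widget from GameInstance server info, replays chat history and refreshes every player's list and count through BP_LobbyPC.
; JoinGame issues server travel to HighRoller (also the fallback) or SkyEdge.
; Logout removes the loop's final index rather than the matched controller, and its "left" message is unwired.
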(event Custom|JoinGame
  (bind _returnvalue (Game|GetPlayerController 0))
  ;[0.15 0.15 0.15 0.5] ServerTravel
  (if (Utilities|Enum|Equal(Enum) (Variables|Default|GetServerMap) "HighRoller")
    (Development|ExecuteConsoleCommand "servertravel/Game/GameMode/Maps/HighRoller" _returnvalue :!label _label)
    (elif (Utilities|Enum|Equal(Enum) (Variables|Default|GetServerMap) "SkyEdge")
      (Development|ExecuteConsoleCommand "servertravel/Game/GameMode/Maps/SkyEdge" _returnvalue)
      (else
        (goto _label))))
  (bind _asbp_game_instance (Utilities|Casting|CastToBP_GameInstance (Game|GetGameInstance)))
  (Default|JoinGame _asbp_game_instance))

(event Custom|UpdateServer
  ;[0.15 0.15 0.15 0.5] UpdateServer
  ;;[0.15 0.15 0.15 0.5] Clear list fro meach player
  (for _array_element (Variables|Default|GetAllPCs)
    (bind _asbp_lobby_pc (Utilities|Casting|CastToBP_LobbyPC _array_element))
    (Default|ClearPlayerList _asbp_lobby_pc)
    ;;[0.15 0.15 0.15 0.5] Add each player to list
    (for (_array_element_2 _array_index) (Variables|Default|GetAllPCs)
      (Default|AddPlayer _asbp_lobby_pc (Utilities|Text|ToText(String) (Class|AdvancedSessionsLibrary|GetPlayerName _array_element_2)) _array_index)))
  ;;[0.15 0.15 0.15 0.5] Update number of players
  (for _array_element_3 (Variables|Default|GetAllPCs)
    (bind _asbp_lobby_pc_2 (Utilities|Casting|CastToBP_LobbyPC _array_element_3))
    (Default|UpdateNumberOfPlayers _asbp_lobby_pc_2 (Utilities|Array|Length (Variables|Default|GetAllPCs)))))

(event Custom|KickPlayer
  (params (Index :type Integer))
  ;[0.15 0.15 0.15 0.5] KickPlayer
  (bind _asbp_lobby_pc (Utilities|Casting|CastToBP_LobbyPC (Utilities|Array|Get(acopy) (Variables|Default|GetAllPCs) Index)))
  (Default|KickPlayer _asbp_lobby_pc))

(event Custom|AddMessageToChatHistory
  (params (Data :type Chat%20Message%20Structure%20Structure))
  ;[0.15 0.15 0.15 0.5] Load Message - History
  (Utilities|Array|Add (Variables|Default|GetMessageLOG) Data))

(event Custom|SendServerMessage
  (params (Message :type String))
  ;[0.15 0.15 0.15 0.5] SnedMessageToEachPlayer
  (bind _asbp_lobby_pc (Utilities|Casting|CastToBP_LobbyPC (Game|GetPlayerController 0)))
  (Default|AddMessagefromServertoEachPlAYER _asbp_lobby_pc Message (Utilities|Struct|MakeSlateColor "(R=1.000000,G=0.000000,B=1.000000,A=1.000000)") true))

(event EventPostLogin
  (params (NewPlayer :type Player%20Controller%20Object%20Reference))
  ;[0.15 0.15 0.15 0.5] Add each Player Controller to list and add server info
  (CallFunction|SendServerMessage (Utilities|String|Append (Class|AdvancedSessionsLibrary|GetPlayerName NewPlayer) "joined"))
  (Networking|SwitchHasAuthority
    (:Authority
      (bind _returnvalue (Utilities|Array|Add (Variables|Default|GetAllPCs) NewPlayer))
      (bind _asbp_game_instance (Utilities|Casting|CastToBP_GameInstance (Game|GetGameInstance)))
      (Variables|Default|SetServerName (Variables|/Game/GameMode/Blueprints/BP_GameInstance.BP_GameInstance_C|GetServerName _asbp_game_instance))
      (Variables|Default|SetServerMap (Variables|/Game/GameMode/Blueprints/BP_GameInstance.BP_GameInstance_C|GetServerMap _asbp_game_instance))
      (Variables|Default|SetServerMode (Variables|/Game/GameMode/Blueprints/BP_GameInstance.BP_GameInstance_C|GetServerMode _asbp_game_instance))
      (Variables|Default|SetServerSlots (Variables|/Game/GameMode/Blueprints/BP_GameInstance.BP_GameInstance_C|GetServerSlots _asbp_game_instance))
      (bind _asbp_lobby_pc (Utilities|Casting|CastToBP_LobbyPC NewPlayer))
      (Default|AddLobbyWB _asbp_lobby_pc (Variables|Default|GetServerName) (Variables|Default|GetServerMap) (Variables|Default|GetServerMode) (Variables|Default|GetServerSlots))
      (CallFunction|UpdateServer)
      ;[0.15 0.15 0.15 0.5] Load Message - History
      (for _array_element (Variables|Default|GetMessageLOG)
        (bind _asbp_lobby_pc_2 (Utilities|Casting|CastToBP_LobbyPC NewPlayer))
        (Default|AddMessagetoChat _asbp_lobby_pc_2 _array_element)))))

(event EventOnLogout
  (params (ExitingController :type Controller%20Object%20Reference))
  (bind _allpcs (Variables|Default|GetAllPCs))
  ;[0.15 0.15 0.15 0.5] RemovePlayerController
  (bind (_array_element _array_index) (Utilities|Array|ForEachLoopwithBreak _allpcs)
    (:LoopBody
      (if (== _array_element ExitingController)
        _))
    (:Completed
      (Utilities|Array|RemoveIndex _allpcs _array_index)
      (CallFunction|UpdateServer))))

(fn ConstructionScript)