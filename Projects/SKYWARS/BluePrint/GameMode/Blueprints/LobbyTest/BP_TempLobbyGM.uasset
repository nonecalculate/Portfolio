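; Multiplayer lobby GameMode for SKYWARS that tracks joined player controllers, syncs the player list and chat history, and server-travels to the chosen map.
; Index-tagged platforms display each player's character, with a delay-polling macro holding placement until platform setup finishes.
; Character selection respawns the platform pawn, records the choice in the GameInstance and resets readiness.
; Lobby info updates recheck whether all players are ready, flagging the host's widget.
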(event Custom|JoinGame
  (bind _returnvalue (Game|GetPlayerController 0))
  ;[0.15 0.15 0.15 0.5] ServerTravel
  (if (Utilities|Enum|Equal(Enum) (Variables|Default|GetServerMap) "Dessert")
    (Development|ExecuteConsoleCommand "servertravel/Game/World/Maps/Desert_A" _returnvalue :!label _label)
    (elif (Utilities|Enum|Equal(Enum) (Variables|Default|GetServerMap) "SkyEdge")
      (Development|ExecuteConsoleCommand "servertravel/Game/GameMode/Maps/SkyEdge" _returnvalue)
      (else
        (goto _label))))
  (bind _asbp_game_instance (Utilities|Casting|CastToBP_GameInstance (Game|GetGameInstance)))
  (Default|JoinGame _asbp_game_instance))

(event Custom|UpdateServer
  ;[0.15 0.15 0.15 0.5] UpdateServer
  ;;[0.15 0.15 0.15 0.5] Clear list fro meach player
  (for _array_element (Variables|Default|GetAllPCs)
    (bind _asbp_temp_lobby_pc (Utilities|Casting|CastToBP_TempLobbyPC _array_element))
    (Utilities|IsValid _asbp_temp_lobby_pc
      (:Is%20Valid
        (Default|ClearPlayerList _asbp_temp_lobby_pc)
        ;;[0.15 0.15 0.15 0.5] Add each player to list
        (for (_array_element_2 _array_index) (Variables|Default|GetAllPCs)
          (Default|AddPlayer _asbp_temp_lobby_pc (Utilities|Text|ToText(String) (Class|AdvancedSessionsLibrary|GetPlayerName _array_element_2)) _array_index)))))
  ;;[0.15 0.15 0.15 0.5] Update number of players
  (for _array_element_3 (Variables|Default|GetAllPCs)
    (bind _asbp_temp_lobby_pc_2 (Utilities|Casting|CastToBP_TempLobbyPC _array_element_3))
    (Default|UpdateNumberOfPlayers _asbp_temp_lobby_pc_2 (Utilities|Array|Length (Variables|Default|GetAllPCs)))))

(event Custom|KickPlayer
  (params (Index :type Integer))
  ;[0.15 0.15 0.15 0.5] KickPlayer
  (bind _asbp_temp_lobby_pc (Utilities|Casting|CastToBP_TempLobbyPC (Utilities|Array|Get(acopy) (Variables|Default|GetAllPCs) Index)))
  (Default|KickPlayer _asbp_temp_lobby_pc))

(event Custom|AddMessageToChatHistory
  (params (Data :type Chat%20Message%20Structure%20Structure))
  ;[0.15 0.15 0.15 0.5] Load Message - History
  (Utilities|Array|Add (Variables|Default|GetMessageLOG) Data))

(event Custom|SendServerMessage
  (params (Message :type String))
  ;[0.15 0.15 0.15 0.5] SnedMessageToEachPlayer
  (bind _asbp_temp_lobby_pc (Utilities|Casting|CastToBP_TempLobbyPC (Game|GetPlayerController 0)))
  (Default|AddMessagefromServertoEachPlayer _asbp_temp_lobby_pc Message (Utilities|Struct|MakeSlateColor "(R=1.000000,G=0.000000,B=1.000000,A=1.000000)") false))

(event EventBeginPlay
  (CallFunction|SetUpPlatforms))

(event EventPostLogin
  (params (NewPlayer :type Player%20Controller%20Object%20Reference))
  ;[0.15 0.15 0.15 0.5] Add each Player Controller to list and add server info
  (CallFunction|SendServerMessage " joined")
  (Networking|SwitchHasAuthority
    (:Authority
      (bind _returnvalue (Utilities|Array|Add (Variables|Default|GetAllPCs) NewPlayer))
      (Utilities|FlowControl|Sequence
        (:then_0
          (bind _asbp_game_instance (Utilities|Casting|CastToBP_GameInstance (Game|GetGameInstance)))
          (Variables|Default|SetServerName (Variables|/Game/GameMode/Blueprints/BP_GameInstance.BP_GameInstance_C|GetServerName _asbp_game_instance))
          (Variables|Default|SetServerMap (Variables|/Game/GameMode/Blueprints/BP_GameInstance.BP_GameInstance_C|GetServerMap _asbp_game_instance))
          (Variables|Default|SetServerMode (Variables|/Game/GameMode/Blueprints/BP_GameInstance.BP_GameInstance_C|GetServerMode _asbp_game_instance))
          (Variables|Default|SetServerSlots (Variables|/Game/GameMode/Blueprints/BP_GameInstance.BP_GameInstance_C|GetServerSlots _asbp_game_instance))
          (bind _asbp_temp_lobby_pc (Utilities|Casting|CastToBP_TempLobbyPC NewPlayer))
          (Default|AddLobbyWB _asbp_temp_lobby_pc (Variables|Default|GetServerName) (Variables|Default|GetServerMap) (Variables|Default|GetServerMode) (Variables|Default|GetServerSlots))
          (CallFunction|UpdateServer)
          ;[0.15 0.15 0.15 0.5] Load Message - History
          (for _array_element (Variables|Default|GetMessageLOG)
            (bind _asbp_temp_lobby_pc_2 (Utilities|Casting|CastToBP_TempLobbyPC NewPlayer))
            (Default|AddMessagetoChat _asbp_temp_lobby_pc_2 _array_element)
            (bind _asbp_game_instance_2 (Utilities|Casting|CastToBP_GameInstance (Game|GetGameInstance)))
            (if (not (> (Variables|/Game/GameMode/Blueprints/BP_GameInstance.BP_GameInstance_C|GetServerSlots _asbp_game_instance_2) _returnvalue))
              (bind _asbp_temp_lobby_gm (Utilities|Casting|CastToBP_TempLobbyGM (Game|GetGameMode)))
              (CallFunction|KickPlayer _asbp_temp_lobby_gm _returnvalue))))
        (:then_1
          (Utilities|IfPlatformsSetUpIsDone
            (:True
              (CallFunction|UpdatePlayersonPlatforms))))))))

(event EventOnLogout
  (params (ExitingController :type Controller%20Object%20Reference))
  (bind _allpcs (Variables|Default|GetAllPCs))
  ;[0.15 0.15 0.15 0.5] RemovePlayerController
  (bind (_array_element _array_index) (Utilities|Array|ForEachLoopwithBreak _allpcs)
    (:LoopBody
      (if (== _array_element ExitingController)
        _))
    (:Completed
      (Utilities|Array|RemoveIndex _allpcs _array_index)
      (CallFunction|UpdateServer)
      (Utilities|IfPlatformsSetUpIsDone
        (:True
          (CallFunction|UpdatePlayersonPlatforms))))))

(fn ConstructionScript)

(fn SetUpPlatforms
  (bind _outactors (Actor|GetAllActorsOfClass "/Game/GameMode/Blueprints/LobbyTest/BP_LobbyPlatform.BP_LobbyPlatform_C"))
  (for _index (range 0 (Utilities|Array|LastIndex _outactors))
    (bind _outactors_2 (Actor|GetAllActorsOfClasswithTag "/Game/GameMode/Blueprints/LobbyTest/BP_LobbyPlatform.BP_LobbyPlatform_C" (Utilities|String|StringToName (Utilities|String|ToString(Integer) _index))))
    (Utilities|Array|Add (Variables|Default|GetPlayerPlatforms) (Utilities|Array|Get(acopy) _outactors_2)))
  (Variables|Default|SetbPlatformsSetUpDone true))

(fn UpdatePlayersonPlatforms
  (for _array_element (Variables|Default|GetAllPCs)
    (LocalVariables|SetLoop_PCAlreadyAdded false)
    (bind _array_element_2 (Utilities|Array|ForEachLoopwithBreak (Variables|Default|GetPlayerPlatforms) :!label _label)
      (:LoopBody
        (if (== (Variables|/Game/GameMode/Blueprints/LobbyTest/BP_LobbyPlatform.BP_LobbyPlatform_C|GetPC _array_element_2) _array_element)
          (LocalVariables|SetLoop_PCAlreadyAdded true)
          (goto _label Break)))
      (:Completed
        (if (not (LocalVariables|GetLoop_PCAlreadyAdded))
          (bind _array_element_3 (Utilities|Array|ForEachLoopwithBreak (Variables|Default|GetPlayerPlatforms) :!label _label_2)
            (:LoopBody
              (Utilities|IsValid (Variables|/Game/GameMode/Blueprints/LobbyTest/BP_LobbyPlatform.BP_LobbyPlatform_C|GetPC _array_element_3)
                (:Is%20Not%20Valid
                  (Default|SpawnCharacter _array_element_3 _array_element)
                  (goto _label_2 Break)))))))))
  (for _array_element_4 (Variables|Default|GetPlayerPlatforms)
    (if (not (Utilities|Array|ContainsItem (Variables|Default|GetAllPCs) (Variables|/Game/GameMode/Blueprints/LobbyTest/BP_LobbyPlatform.BP_LobbyPlatform_C|GetPC _array_element_4)))
      (Default|Clear _array_element_4))))

(fn UpdatePlayerLobbyInfo
  (params (RequestingPC :type Player%20Controller%20Object%20Reference))
  (bind _playername (Class|AdvancedSessionsLibrary|GetPlayerName RequestingPC))
  (bind _asbp_temp_lobby_pc (Utilities|Casting|CastToBP_TempLobbyPC RequestingPC))
  (bind _playerstate (Variables|/Script/Engine.Controller|GetPlayerState RequestingPC))
  (bind _returnvalue (Utilities|Text|ToText(String) _playername))
  (bind _playerlobbyinfopc (Variables|/Game/GameMode/Blueprints/LobbyTest/BP_TempLobbyPC.BP_TempLobbyPC_C|GetPlayerLobbyInfoPC _asbp_temp_lobby_pc))
  (bind _bready (Utilities|Struct|BreakST_PlayerLobbyInfo _playerlobbyinfopc))
  (bind _st_playerlobbyinfo (Utilities|Struct|MakeST_PlayerLobbyInfo RequestingPC _returnvalue _bready _playerstate))
  (for _array_element (Variables|Default|GetPlayerPlatforms)
    (if (== (Variables|/Game/GameMode/Blueprints/LobbyTest/BP_LobbyPlatform.BP_LobbyPlatform_C|GetPC _array_element) RequestingPC)
      (bind _asbp_sw_lobby_dubu (Utilities|Casting|CastToBP_SW_LobbyDubu (Variables|/Game/GameMode/Blueprints/LobbyTest/BP_LobbyPlatform.BP_LobbyPlatform_C|GetCurrentCharacter _array_element))
        (:then
          (Default|UpdatePlayerLobbyInfo _asbp_sw_lobby_dubu _st_playerlobbyinfo))
        (:CastFailed
          (bind _asbp_sw_lobby_brall (Utilities|Casting|CastToBP_SW_LobbyBrall (Variables|/Game/GameMode/Blueprints/LobbyTest/BP_LobbyPlatform.BP_LobbyPlatform_C|GetCurrentCharacter _array_element)))
          (Default|UpdatePlayerLobbyInfo _asbp_sw_lobby_brall _st_playerlobbyinfo)))
      (CallFunction|CheckifEnoughPlayersAreReady)
      (return)))
  (Default|TryAgainUpdatingLobbyInfo (.AsBP%20Temp%20Lobby%20PC (Utilities|Casting|CastToBP_TempLobbyPC RequestingPC))))

(fn SelectCharacterClassbyIndex
  (params (PC :type Player%20Controller%20Object%20Reference) (Character%20Index :type Integer))
  (for _array_element (Variables|Default|GetPlayerPlatforms)
    (bind _output_get (LocalVariables|SetLoopPlatformRef _array_element))
    (if (== (Variables|/Game/GameMode/Blueprints/LobbyTest/BP_LobbyPlatform.BP_LobbyPlatform_C|GetPC _output_get) PC)
      (Utilities|FlowControl|Sequence
        (:then_0
          (Utilities|IsValid (Variables|/Game/GameMode/Blueprints/LobbyTest/BP_LobbyPlatform.BP_LobbyPlatform_C|GetCurrentCharacter (LocalVariables|GetLoopPlatformRef))
            (:Is%20Valid
              (Actor|DestroyActor (Variables|/Game/GameMode/Blueprints/LobbyTest/BP_LobbyPlatform.BP_LobbyPlatform_C|GetCurrentCharacter (LocalVariables|GetLoopPlatformRef))))))
        (:then_1
          (bind _output_get_2 (LocalVariables|SetSelectedCharacterClass (Utilities|Array|Get(acopy) (Variables|Default|GetAvailableCharacterClass) Character%20Index)))
          (bind _returnvalue (Game|SpawnActorfromClass _output_get_2 (Transformation|GetWorldTransform (Variables|/Game/GameMode/Blueprints/LobbyTest/BP_LobbyPlatform.BP_LobbyPlatform_C|GetPlayerSpawnTransform (LocalVariables|GetLoopPlatformRef))) "Undefined" "MultiplyWithRoot" 0 0))
          (bind _output_get_3 (Variables|/Game/GameMode/Blueprints/LobbyTest/BP_LobbyPlatform.BP_LobbyPlatform_C|SetCurrentCharacter (LocalVariables|GetLoopPlatformRef) _returnvalue))
          (Collision|SetActorEnableCollision _output_get_3 false)
          (LocalVariables|SetSelectedCharacterClass (Utilities|Array|Get(acopy) (Variables|Default|GetAvailiableToSelectedCharacter) Character%20Index))
          (Utilities|Map|Add (Variables|/Game/GameMode/Blueprints/BP_GameInstance.BP_GameInstance_C|GetSelectedCharacterOfAllPlayers (.AsBP%20Game%20Instance (Utilities|Casting|CastToBP_GameInstance (Game|GetGameInstance)))) (PlayerState|GetPlayerName (Variables|/Script/Engine.Controller|GetPlayerState PC)) (LocalVariables|GetSelectedCharacterClass))
          (Utilities|Struct|SetmembersinST_PlayerLobbyInfo (Variables|/Game/GameMode/Blueprints/LobbyTest/BP_TempLobbyPC.BP_TempLobbyPC_C|GetPlayerLobbyInfoPC (.AsBP%20Temp%20Lobby%20PC (Utilities|Casting|CastToBP_TempLobbyPC PC))) false)
          (CallFunction|UpdatePlayerLobbyInfo PC)
          (return))))))

(fn CheckifEnoughPlayersAreReady
  (LocalVariables|SetbAllPlayersReady true)
  (for _array_element (Variables|Default|GetAllPCs)
    (bind _asbp_temp_lobby_pc (Utilities|Casting|CastToBP_TempLobbyPC _array_element))
    (if (not (.bReady (Utilities|Struct|BreakST_PlayerLobbyInfo (Variables|/Game/GameMode/Blueprints/LobbyTest/BP_TempLobbyPC.BP_TempLobbyPC_C|GetPlayerLobbyInfoPC _asbp_temp_lobby_pc))))
      (LocalVariables|SetbAllPlayersReady false)))
  (bind _asbp_temp_lobby_pc_2 (Utilities|Casting|CastToBP_TempLobbyPC (Game|GetPlayerController 0)))
  (Variables|/Game/GameMode/UMG/TempUMG/UMG_TempLobby.UMG_TempLobby_C|SetbEnoughPlayersReady (Variables|/Game/GameMode/Blueprints/LobbyTest/BP_TempLobbyPC.BP_TempLobbyPC_C|GetLobbyWB _asbp_temp_lobby_pc_2) (LocalVariables|GetbAllPlayersReady)))