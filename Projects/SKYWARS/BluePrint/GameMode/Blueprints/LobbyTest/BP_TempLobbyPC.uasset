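; Lobby player controller for a multiplayer session, owning the lobby widget with player list, chat and server info, and swapping it for a loading screen.
; Name, ready toggle (R key) and character choices go through BP_TempLobbyGM, which handles lobby info and character selection.
; Chat messages are relayed to every controller in the game mode's list and saved to its history.
; Kicking leaves the session through the game instance.
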(event Custom|AddLobbyWB
  (params (ServerName :type String) (ServerMap :type String) (ServerMode :type String) (ServerSlots :type Integer))
  (Variables|Default|SetbShowMouseCursor true)
  (bind _returnvalue (UserInterface|CreateWidget "/Game/GameMode/UMG/TempUMG/UMG_TempLobby.UMG_TempLobby_C" 0 (Utilities|Text|ToText(String) ServerName) (Utilities|Text|ToText(String) ServerMap) (Utilities|Text|ToText(String) ServerMode) ServerSlots))
  (bind _output_get (Variables|Default|SetLobbyWB _returnvalue))
  (UserInterface|Viewport|AddtoViewport _output_get 1))

(event Custom|LoadingScreen
  (Widget|RemovefromParent (Variables|Default|GetLobbyWB))
  (bind _returnvalue (UserInterface|CreateWidget "/Game/GameMode/UMG/UMG_LoadingScreen.UMG_LoadingScreen_C" self))
  (UserInterface|Viewport|AddtoViewport _returnvalue 0))

(event Custom|SetPlayerNameOnServer
  (params (PlayerName :type Text))
  (Utilities|Struct|SetmembersinST_PlayerLobbyInfo (Variables|Default|GetPlayerLobbyInfoPC) PlayerName)
  (bind _asbp_temp_lobby_gm (Utilities|Casting|CastToBP_TempLobbyGM (Game|GetGameMode)))
  (Default|UpdatePlayerLobbyInfo _asbp_temp_lobby_gm self))

(event Custom|ToggleReadyStatusOnServer
  (bind _playerlobbyinfopc (Variables|Default|GetPlayerLobbyInfoPC))
  (Utilities|Struct|SetmembersinST_PlayerLobbyInfo _playerlobbyinfopc (not (.bReady (Utilities|Struct|BreakST_PlayerLobbyInfo _playerlobbyinfopc))))
  (bind _asbp_temp_lobby_gm (Utilities|Casting|CastToBP_TempLobbyGM (Game|GetGameMode)))
  (Default|UpdatePlayerLobbyInfo _asbp_temp_lobby_gm self))

(event Custom|ServerSelectCharacterByEnum
  (params (SelectedCharacterType :type ECharacterType%20Enum :default "START"))
  (bind _asbp_temp_lobby_gm (Utilities|Casting|CastToBP_TempLobbyGM (Game|GetGameMode)))
  (Default|SelectCharacterClassbyIndex _asbp_temp_lobby_gm self (- (Math|Conversions|ToInteger(Byte) SelectedCharacterType) 1)))

(event Custom|AddPlayer
  (params (Player :type Text) (PlayerIndex :type Integer))
  (Default|AddPlayertoList (Variables|Default|GetLobbyWB) Player PlayerIndex))

(event Custom|ClearPlayerList
  (Default|ClearPlayerList (Variables|Default|GetLobbyWB)))

(event Custom|KickPlayer
  (bind _asbp_game_instance (Utilities|Casting|CastToBP_GameInstance (Game|GetGameInstance)))
  (Default|LeaveSession _asbp_game_instance))

(event Custom|UpdateNumberOfPlayers
  (params (CurrentPlayers :type Integer))
  (Variables|/Game/GameMode/UMG/TempUMG/UMG_TempLobby.UMG_TempLobby_C|SetCurrentPlayers (Variables|Default|GetLobbyWB) CurrentPlayers))

(event Custom|AddMessageFromServerToEachPlayer
  (params (Message :type String) (Color :type Slate%20Color%20Structure) (isServerMessage? :type Boolean))
  (bind _self self)
  (bind _playername (Class|AdvancedSessionsLibrary|GetPlayerName _self))
  (bind _chatmessagestructure (Utilities|Struct|MakeChatMessageStructure _playername Message Color isServerMessage?))
  (bind _asbp_temp_lobby_gm (Utilities|Casting|CastToBP_TempLobbyGM (Game|GetGameMode)))
  (for _array_element (Variables|/Game/GameMode/Blueprints/LobbyTest/BP_TempLobbyGM.BP_TempLobbyGM_C|GetAllPCs _asbp_temp_lobby_gm)
    (bind _asbp_temp_lobby_pc (Utilities|Casting|CastToBP_TempLobbyPC _array_element))
    (CallFunction|AddMessagetoChat _asbp_temp_lobby_pc _chatmessagestructure))
  (bind _asbp_temp_lobby_gm_2 (Utilities|Casting|CastToBP_TempLobbyGM (Game|GetGameMode)))
  (Default|AddMessagetoChatHistory _asbp_temp_lobby_gm_2 _chatmessagestructure))

(event Custom|AddMessageToChat
  (params (ChatMessageStructure :type Chat%20Message%20Structure%20Structure))
  (bind _lobbywb (Variables|Default|GetLobbyWB))
  (Utilities|IsValid _lobbywb
    (:Is%20Valid
      (Default|AddChildtoChat (Variables|/Game/GameMode/UMG/TempUMG/UMG_TempLobby.UMG_TempLobby_C|GetUMG_TempChatWindow _lobbywb) ChatMessageStructure))))

(event Custom|TryAgainUpdatingLobbyInfo
  (Utilities|FlowControl|Delay 0.1)
  (bind _asbp_temp_lobby_gm (Utilities|Casting|CastToBP_TempLobbyGM (Game|GetGameMode)))
  (Default|UpdatePlayerLobbyInfo _asbp_temp_lobby_gm self))

(event Custom|SelectCharacterOnServer
  (Utilities|FlowControl|MultiGate false true 0
    (:Out%200
      (Default|SelectCharacterClassbyIndex (Variables|Default|GetLobbyGM_Ref) self))
    (:Out%201
      (Default|SelectCharacterClassbyIndex (Variables|Default|GetLobbyGM_Ref) self 1))))

(event EventBeginPlay
  (CallFunction|SetUp)
  (Variables|Default|SetLobbyGM_Ref (.AsBP%20Temp%20Lobby%20GM (Utilities|Casting|CastToBP_TempLobbyGM (Game|GetGameMode)))))

(event Input|KeyboardEvents|R
  (params (Key :type Key%20Structure :default "None"))
  (:Pressed
    (CallFunction|ToggleReadyStatusonServer)))

(fn ConstructionScript)

(fn SetUp
  (if (Pawn|IsLocalPlayerController)
    (Variables|Default|SetbShowMouseCursor true)
    (Input|SetInputModeGameandUI self 0 "DoNotLock" false false)
    (UserInterface|CreateWidget "/Game/GameMode/UMG/TempUMG/UMG_TempLobby.UMG_TempLobby_C")
    (CallFunction|SetPlayerNameonServer (.PlayerName (Utilities|Struct|BreakST_PlayerLobbyInfo (Variables|Default|GetPlayerLobbyInfoPC))))))