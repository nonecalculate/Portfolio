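; Lobby actor that shows a player's lobby info on its LobbyInfo widget component.
; UpdatePlayerLobbyInfo sets the PlayerLobbyInfo variable, whose OnRep passes it to the UMG_PlayerLobbyInfo widget and makes the component visible.
; If the widget is not yet valid, the OnRep retries itself on a short timer.
; The event graph and construction script hold no logic.
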(event EventBeginPlay)

(event Collision|EventActorBeginOverlap
  (params (OtherActor :type Actor%20Object%20Reference)))

(event EventTick
  (params (DeltaSeconds :type Float%20%28single-precision%29)))

(fn ConstructionScript)

(fn UpdatePlayerLobbyInfo
  (params (PlayerLobbyInfo :type ST%20Player%20Lobby%20Info%20Structure))
  (Variables|Default|SetPlayerLobbyInfo PlayerLobbyInfo))

(fn OnRepPlayerLobbyInfo
  (bind _lobbyinfo (Variables|Default|GetLobbyInfo))
  (bind _returnvalue (UserInterface|GetWidget _lobbyinfo))
  (Utilities|IsValid _returnvalue
    (:Is%20Valid
      (bind _asumg_player_lobby_info (Utilities|Casting|CastToUMG_PlayerLobbyInfo _returnvalue))
      (Default|Update _asumg_player_lobby_info (Variables|Default|GetPlayerLobbyInfo))
      (Rendering|SetVisibility (Variables|Default|GetLobbyInfo) true false))
    (:Is%20Not%20Valid
      (Utilities|Time|SetTimerbyFunctionName 0 "OnRep_PlayerLobbyInfo" 0.1))))