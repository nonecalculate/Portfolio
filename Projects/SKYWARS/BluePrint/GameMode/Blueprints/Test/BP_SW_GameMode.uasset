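; BP_SW_GameMode is a SKYWARS game mode that handles per-player pawn selection, lobby creation and result display.
; It overrides GetDefaultPawnClassForController to look up each player's chosen character by player name in BP_GameInstance, falling back to BP_SW_Dubu.
; CreateSession passes the game instance's stored server settings to CreateLobby.
; PopUpResult opens the result window on each controller in PlayerControllers.
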(event EventPopUpResult
  (for _array_element (Variables|Default|GetPlayerControllers)
    (bind _asbp_sw_player_controller (Utilities|Casting|CastToBP_SW_PlayerController _array_element))
    (Default|PopUpResultWindow _asbp_sw_player_controller)))

(event EventCreateSession
  (bind _asbp_game_instance (Utilities|Casting|CastToBP_GameInstance (Game|GetGameInstance)))
  (Default|CreateLobby _asbp_game_instance (Variables|/Game/GameMode/Blueprints/BP_GameInstance.BP_GameInstance_C|GetServerName _asbp_game_instance) (Variables|/Game/GameMode/Blueprints/BP_GameInstance.BP_GameInstance_C|GetServerMap _asbp_game_instance) (Variables|/Game/GameMode/Blueprints/BP_GameInstance.BP_GameInstance_C|GetServerMode _asbp_game_instance) (Variables|/Game/GameMode/Blueprints/BP_GameInstance.BP_GameInstance_C|GetServerSlots _asbp_game_instance) (Variables|/Game/GameMode/Blueprints/BP_GameInstance.BP_GameInstance_C|GetServerMethod_LAN _asbp_game_instance) (Variables|/Game/GameMode/Blueprints/BP_GameInstance.BP_GameInstance_C|GetHas%20Password? _asbp_game_instance) (Variables|/Game/GameMode/Blueprints/BP_GameInstance.BP_GameInstance_C|GetPassword _asbp_game_instance)))

(fn ConstructionScript)

(fn GetDefaultPawnClassforController
  (params (InController :type Controller%20Object%20Reference))
  (bind _returnvalue (Game|GetGameInstance))
  (bind _playerstate (Variables|/Script/Engine.Controller|GetPlayerState InController))
  (bind _returnvalue_2 (PlayerState|GetPlayerName _playerstate))
  (bind _asbp_game_instance (Utilities|Casting|CastToBP_GameInstance _returnvalue))
  (bind _selectedcharacterofallplayers (Variables|/Game/GameMode/Blueprints/BP_GameInstance.BP_GameInstance_C|GetSelectedCharacterOfAllPlayers _asbp_game_instance))
  (bind _value (Utilities|Map|Find _selectedcharacterofallplayers _returnvalue_2))
  (if (Utilities|IsValidClass _value)
    (return _value)
    (else
      (return "/Game/Characters/Dubu/BP_SW_Dubu.BP_SW_Dubu_C"))))